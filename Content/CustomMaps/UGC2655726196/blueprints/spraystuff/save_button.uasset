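; Spray tester button that records weapon recoil patterns; tracking starts shortly after play begins and resets on point damage.
; AddDataPoint stores timed hit positions relative to the first, logs them as text and redraws them rescaled on a spray canvas.
; A second canvas shows the inverted pattern joined by a curve, as recoil compensation.
; Stats show average fire rate and bullet speed, cached per bullet name by OnActorOverlap.
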(event EventBeginPlay
  (Utilities|FlowControl|Delay 0.5)
  (CallFunction|StartTracking))

(event Game|Damage|EventPointDamage
  (params (Damage :type Float%20%28single-precision%29) (DamageType :type Damage%20Type%20Object%20Reference) (HitLocation :type Vector :default "0, 0, 0") (HitNormal :type Vector :default "0, 0, 0") (HitComponent :type Primitive%20Component%20Object%20Reference) (BoneName :type Name :default "None") (ShotFromDirection :type Vector :default "0, 0, 0") (InstigatedBy :type Controller%20Object%20Reference) (DamageCauser :type Actor%20Object%20Reference) (HitInfo :type Hit%20Result%20Structure%20%28by%20ref%29))
  (CallFunction|StopTracking)
  (CallFunction|StartTracking)
  (bind _gamelogic (Utilities|GetGameLogic)
    (:ExecOut
      (Default|Print _gamelogic "Spray tester reset."))))

(fn ConstructionScript
  (Variables|Default|Settracking false))

(fn StartTracking
  (Utilities|Array|Clear (Variables|Default|Getdata))
  (Variables|Default|Settracking true)
  (Variables|Default|SettotalTime 0.0)
  (Utilities|Map|Clear (Variables|Default|GetbulletVelocityMap))
  (Variables|Default|SetlastBullet "")
  (Rendering|Material|SetMaterial (Variables|Debug|GetStaticMeshComponent) 0 "/Game/CustomMaps/UGC2655726196/mats/solid_red.solid_red")
  (Rendering|Components|TextRender|SetText (Variables|Default|GetdataDisplay) (Utilities|Text|ToText(String) (Utilities|String|MakeLiteralString "Recording... 
")))
  (CallFunction|UpdateStatsDisplay)
  (return))

(fn StopTracking
  (Variables|Default|Settracking false)
  (Rendering|Material|SetMaterial (Variables|Debug|GetStaticMeshComponent) 0 "/Game/CustomMaps/UGC2655726196/mats/solid_green.solid_green")
  (CallFunction|AddTextLine "Done.")
  (return))

(fn AddDataPoint
  (params (pos :type Vector) (time :type Float%20%28single-precision%29) (bulletName :type String))
  (bind _compensation_canvas (Variables|Default|Getcompensation_canvas))
  (if (Variables|Default|Gettracking)
    (Utilities|FlowControl|Sequence
      (:then_0
        ;[1 1 1] Set the new point to be the input pos relative to the first point (offset) in the sequence)
        (if (== (Utilities|Array|Length (Variables|Default|Getdata)) 0)
          (Variables|Default|Setoffset pos)
          (LocalVariables|SetnewPoint "0, 0, 0")
          (Variables|Default|Setscale 1.0)
          (else
            (LocalVariables|SetnewPoint (* (- pos (Variables|Default|Getoffset)) "1.000000,1.000000,1.000000")))))
      (:then_1
        ;[1 1 1] Append Point to the Data Array
        (Utilities|Array|AppendArray (Variables|Default|Getdata) (Utilities|Array|MakeArray (Math|Vector4|MakeVector4 (.x (LocalVariables|GetnewPoint)) (.y (LocalVariables|GetnewPoint)) (.z (LocalVariables|GetnewPoint)) time)))
        (Variables|Default|Setscale (Math|Float|Max(Float) (.z (LocalVariables|GetnewPoint)) (Variables|Default|Getscale))))
      (:then_2
        ;[1 1 1] Print Point to Display
        (CallFunction|AddTextLine (Utilities|String|Append "<" (Utilities|String|ToString(Float) (.x (LocalVariables|GetnewPoint))) ", " (Utilities|String|ToString(Float) (.z (LocalVariables|GetnewPoint))) ">: " (Utilities|String|ToString(Float) time) "s 
")))
      (:then_3
        ;[1 1 1] Draw rescaled points on the canvas
        (Default|Clear (Variables|Default|Getspray_canvas))
        (for _array_element (Variables|Default|Getdata)
          (Default|Draw (Variables|Default|Getspray_canvas) "/Game/CustomMaps/UGC2655726196/mats/canvas/hit_marker.hit_marker" 16.0 (Utilities|RescalePoint _array_element))))
      (:then_4
        ;[1 1 1] Draw compensation points on the other canvas
        (Utilities|FlowControl|Sequence
          (:then_0
            (LocalVariables|SetsprayCurve (Utilities|Array|MakeArray))
            (Default|Clear _compensation_canvas)
            (for _array_element_2 (Variables|Default|Getdata)
              (Default|Draw (Variables|Default|Getcompensation_canvas) "/Game/CustomMaps/UGC2655726196/mats/canvas/hit_marker.hit_marker" 16.0 (- "(X=1.000000,Y=1.000000)" (Utilities|RescalePoint _array_element_2)))
              (Utilities|Array|AppendArray (LocalVariables|GetsprayCurve) (Utilities|Array|MakeArray (- "(X=1.000000,Y=1.000000)" (Utilities|RescalePoint _array_element_2))))))
          (:then_1
            (Default|DrawCurve _compensation_canvas (LocalVariables|GetsprayCurve) 4.0))))
      (:then_5
        ;[1 1 1] Calculate Stats
        (if (not (<= (Utilities|Array|Length (Variables|Default|Getdata)) 1))
          (Variables|Default|SettotalTime (+ (Variables|Default|GettotalTime) time))
          (Variables|Default|SetlastBullet bulletName)
          (CallFunction|UpdateStatsDisplay))))))

(fn AddTextLine
  (params (line :type String))
  (Rendering|Components|TextRender|SetText (Variables|Default|GetdataDisplay) (Utilities|Text|ToText(String) (Utilities|String|Append (Utilities|String|ToString(Text) (Variables|/Script/Engine.TextRenderComponent|GetText (Variables|Default|GetdataDisplay))) " 
" line)))
  (return))

(fn UpdateStatsDisplay
  (bind _totaltime (Variables|Default|GettotalTime))
  (bind _data (Variables|Default|Getdata))
  (bind _bulletvelocitymap (Variables|Default|GetbulletVelocityMap))
  (bind _lastbullet (Variables|Default|GetlastBullet))
  (bind _returnvalue (Utilities|Array|Length _data))
  (bind (_value _returnvalue_2) (Utilities|Map|Find _bulletvelocitymap _lastbullet))
  (bind _returnvalue_3 (- _returnvalue 1))
  (bind _returnvalue_4 (Math|Conversions|ToFloat(Integer) _returnvalue_3))
  (bind _returnvalue_5 (/ _returnvalue_4 _totaltime))
  (LocalVariables|Settmp "Avg Fire Rate: ")
  (if (<= _returnvalue 1)
    (LocalVariables|Settmp (Utilities|String|Append (LocalVariables|Gettmp) "?"))
    (else
      (bind _output_get (LocalVariables|Settmp (Utilities|String|Append (LocalVariables|Gettmp) (Utilities|String|ToString(Float) (Utilities|Round2dec _returnvalue_5)) " rps" " (" (Utilities|String|ToString(Float) (Utilities|Round2dec (* _returnvalue_5 6e+01))) " rpm)")))))
  (LocalVariables|Settmp (Utilities|String|Append _output_get " 
Bullet Speed: "))
  (if _returnvalue_2
    (bind _output_get_2 (LocalVariables|Settmp (Utilities|String|Append (LocalVariables|Gettmp) (Utilities|String|ToString(Float) (Utilities|Round2dec _value)) " m/s")))
    (else
      (LocalVariables|Settmp (Utilities|String|Append (LocalVariables|Gettmp) "?"))))
  (Rendering|Components|TextRender|SetText (Variables|Default|GetstatsDisplay) (Utilities|Text|ToText(String) _output_get_2)))

(fn OnActorOverlap
  (params (actor :type Actor%20Object%20Reference))
  (Utilities|Map|Add (Variables|Default|GetbulletVelocityMap) (Utilities|GetObjectName actor) (/ (Math|Vector|VectorLength (Transformation|GetVelocity actor)) 1e+02)))