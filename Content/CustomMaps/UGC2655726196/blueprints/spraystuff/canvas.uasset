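; Paintable canvas actor in a spray-paint map that shows runtime drawing on its static mesh.
; BeginPlay creates a render target, clears it to white and feeds it into a dynamic material on the mesh.
; Draw stamps a textured brush material centered on a location, while DrawCurve joins points with colored lines.
; Both draw through the render target's canvas, using ScaleToDraw to convert positions to canvas space.
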(event EventBeginPlay
  (Utilities|FlowControl|Sequence
    (:then_0
      (bind _returnvalue (Rendering|CreateRenderTarget2D 1024 1024 "RTF_RGBA16f"))
      (Variables|Default|SetrenderTarget _returnvalue)
      (CallFunction|Clear))
    (:then_1
      (bind _returnvalue_2 (Rendering|Material|CreateDynamicMaterialInstance "/Game/CustomMaps/UGC2655726196/mats/canvas/canvas_base.canvas_base" "None" :!class /Script/Engine.KismetMaterialLibrary))
      (Rendering|Material|SetTextureParameterValue _returnvalue_2 "RenderTarget" (Variables|Default|GetrenderTarget))
      (Rendering|Material|SetMaterial (Variables|Debug|GetStaticMeshComponent) 0 _returnvalue_2))
    (:then_2
      (bind _returnvalue_3 (Rendering|Material|CreateDynamicMaterialInstance "/Game/CustomMaps/UGC2655726196/mats/canvas/canvas_brush.canvas_brush" "None" :!class /Script/Engine.KismetMaterialLibrary))
      (Variables|Default|SetbrushMaterial _returnvalue_3))))

(fn ConstructionScript)

(fn Clear
  (Rendering|ClearRenderTarget2D (Variables|Default|GetrenderTarget) "(R=1.000000,G=1.000000,B=1.000000,A=1.000000)"))

(fn Draw
  (params (BrushTexture :type Texture%202D%20Object%20Reference) (BrushSize :type Float%20%28single-precision%29) (DrawLocation :type Vector%202D%20Structure))
  (Utilities|FlowControl|Sequence
    (:then_0
      (Rendering|Material|SetTextureParameterValue (Variables|Default|GetbrushMaterial) "BrushTexture" BrushTexture))
    (:then_1
      (bind (_canvas _size _context) (Rendering|BeginDrawCanvastoRenderTarget (Variables|Default|GetrenderTarget)))
      (Canvas|DrawMaterial :self _canvas :RenderMaterial (Variables|Default|GetbrushMaterial) :ScreenPosition (- (Utilities|ScaletoDraw DrawLocation _size) (/ BrushSize 2.0)) :ScreenSize (Math|Vector2D|MakeVector2D BrushSize BrushSize))
      (Rendering|EndDrawCanvastoRenderTarget _context))))

(fn DrawCurve
  (params (points :type Array%20of%20Vector%202D%20Structures) (strokeWidth :type Float%20%28single-precision%29) (color :type Linear%20Color%20Structure))
  (Utilities|FlowControl|Sequence
    (:then_0
      (bind (_canvas _size _context) (Rendering|BeginDrawCanvastoRenderTarget (Variables|Default|GetrenderTarget)))
      (LocalVariables|SetcanvasSize _size))
    (:then_1
      (for (_array_element _array_index) points
        (if (== _array_index 0)
          _
          (else
            (Class|Canvas|DrawLine _canvas (LocalVariables|GetlastPoint) (Utilities|ScaletoDraw _array_element (LocalVariables|GetcanvasSize)) strokeWidth color)))
        (LocalVariables|SetlastPoint (Utilities|ScaletoDraw _array_element (LocalVariables|GetcanvasSize)))))
    (:then_2
      (Rendering|EndDrawCanvastoRenderTarget _context))))