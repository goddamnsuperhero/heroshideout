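; Server portal actor for a Pavlov VR custom map that shows live information about one configured game server.
; When the local player pawn overlaps it, a self-resetting DoOnce requests the Pavlov master server list over HTTP.
; The response handler matches IP and port, then writes name, map and slot counts to display text.
; ConnectToServer builds an "open" console command, but nothing here calls it.
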(event Custom|OnResponseRecieved
  (params (RequestObject :type Json%20Utils%20Request%20Object%20Reference) (bSuccessful :type Boolean))
  (bind _array_element (Utilities|Array|ForEachLoopwithBreak (.ReturnValue (Class|JsonUtilsObj|GetArrayasObjects (.ReturnValue (Class|JsonUtilsRequest|GetResponseasJson RequestObject)) "servers")) :!label _label)
    (:LoopBody
      (if (and (Utilities|Enum|Equal(Enum) (.StringValue (Class|JsonUtilsObj|GetStringField _array_element "ip")) (Variables|Default|Getserver_ip)) (Utilities|Enum|Equal(Enum) (.StringValue (Class|JsonUtilsObj|GetStringField _array_element "port")) (Variables|Default|Getserver_port)))
        (Variables|Default|Setserver_name (.StringValue (Class|JsonUtilsObj|GetStringField _array_element "name")))
        (Variables|Default|Setserver_map_name (.StringValue (Class|JsonUtilsObj|GetStringField _array_element "mapLabel")))
        (Variables|Default|Setserver_max_slots (.NumberValue (Class|JsonUtilsObj|GetIntField _array_element "maxSlots")))
        (Variables|Default|Setserver_cur_slots (.NumberValue (Class|JsonUtilsObj|GetIntField _array_element "slots")))
        (CallFunction|UpdateDisplay)
        (goto _label Break)))))

(event Collision|EventActorBeginOverlap
  (params (OtherActor :type Actor%20Object%20Reference))
  (Networking|SwitchHasAuthority
    (:Authority
      _)
    (:Remote
      _))
  (if (== OtherActor (Game|Player|GetPlayerPawn 0))
    (Utilities|FlowControl|DoOnce false :!label _label
      (:Completed
        (Utilities|FlowControl|Sequence
          (:then_0
            (CallFunction|UpdateServerInfo)
            (Utilities|FlowControl|Delay 2.0)
            (Development|PrintString (Variables|Default|Getserver_name)))
          (:then_1
            (Utilities|FlowControl|Delay 5.0)
            (goto _label Reset)))))))

(fn ConstructionScript)

(fn UpdateServerInfo
  (bind _output_get (Variables|Default|Setrequest (Class|JsonUtilsLib|MakeHttpRequest)))
  (Utilities|IsValid _output_get
    (:Is%20Valid
      (Class|JsonUtilsRequest|AddRequestHeader _output_get "version" "0.70.0")
      (Class|JsonUtilsRequest|SetURL _output_get "ms.pavlov-vr.com/v1/servers")
      (EventDispatchers|BindEventtoOnResponseReceived _output_get (EventDispatchers|CreateEvent :!event Custom|OnResponseRecieved))
      (Class|JsonUtilsRequest|ProcessRequest _output_get))))

(fn ConnecttoServer
  (Development|ExecuteConsoleCommand (Utilities|String|Append "open " (Variables|Default|Getserver_ip) ":" (Variables|Default|Getserver_port)) 0))

(fn UpdateDisplay
  (Rendering|Components|TextRender|SetText (Variables|Default|GetdisplayText) (Utilities|Text|ToText(String) (Utilities|String|Append (Variables|Default|Getserver_name) " 
" (Variables|Default|Getserver_map_name) " 
" (Utilities|String|ToString(Integer) (Variables|Default|Getserver_cur_slots)) " / " (Utilities|String|ToString(Integer) (Variables|Default|Getserver_max_slots))))))