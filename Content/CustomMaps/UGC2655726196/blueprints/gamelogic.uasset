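; Game logic actor for a Pavlov custom map that, one second after BeginPlay, destroys any TeamDeathMatchGameMode_C actors, found by scanning all actors by class display name.
; An unconnected chain would configure a teamless, non-scoring auto-respawn mode with no fall damage, unlimited-range buying and large cash grants.
; Helper functions send server chat messages and, gated by a debug setting, dump player status or unique actor class names.
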(event EventBeginPlay
  (Utilities|FlowControl|Delay 1.0)
  (bind _actors (CallFunction|FindAllActorswithClassName "TeamDeathMatchGameMode_C"))
  (for _array_element _actors
    (Actor|DestroyActor _array_element)))

(fn ConstructionScript)

(fn Print
  (params (line :type String))
  (Default|Print (Variables|Default|GetplayerModifier) line)
  (Class|PavlovLibrary|SendAllMsg (Utilities|Struct|MakeMessage "Server" (Utilities|Text|ToText(String) line))))

(fn PrintDebug
  (params (line :type String))
  (if (.Value (Utilities|Map|Find (Variables|Default|GetboolSettings) "NewEnumerator4"))
    (CallFunction|Print line)))

(fn FindAllActorswithClassName
  (params (className :type String))
  (bind _tmp (LocalVariables|Gettmp))
  (bind _outactors (Actor|GetAllActorsOfClass "/Script/Engine.Actor"))
  (for _array_element _outactors
    (if (Utilities|Enum|Equal(Enum) (Utilities|GetClassDisplayName (Utilities|GetClass _array_element)) className)
      (Utilities|Array|AppendArray _tmp (Utilities|Array|MakeArray _array_element))))
  (return _tmp))

(fn PrintPlayerState
  (params (pawn :type Pawn%20Object%20Reference))
  (bind _playerstatus (Class|PavlovProxyStatics|GetPavlovPlayerStatusbyPawn pawn))
  (CallFunction|PrintDebug (Utilities|String|Append (Utilities|String|Append "SID: " (.steamid _playerstatus) "; Cash: " (Utilities|String|ToString(Integer) (.cash _playerstatus)) "; Score: " (Utilities|String|ToString(Integer) (.score _playerstatus)) "; 
  Team ID: " (Utilities|String|ToString(Integer) (.teamid _playerstatus)) "; Health: " (Utilities|String|ToString(Integer) (.health _playerstatus)) "; Armor: " (Utilities|String|ToString(Integer) (.armour _playerstatus)) "; Helmet: " (Utilities|String|ToString(Boolean) (.bhelmet _playerstatus)) "; Can Buy: " (Utilities|String|ToString(Boolean) (.bcanbuy _playerstatus)) "; 
  Dead: " (Utilities|String|ToString(Boolean) (.bdead _playerstatus)) "; Crouch: " (Utilities|String|ToString(Boolean) (.bcrouching _playerstatus)) "; Gagged: " (Utilities|String|ToString(Boolean) (.bgagged _playerstatus)) "; Right Handed:" (Utilities|String|ToString(Boolean) (.brighthanded _playerstatus))) "; 
  Dead Time: " (Utilities|String|ToString(Float) (.deadtime _playerstatus)) "; Alive Time: " (Utilities|String|ToString(Float) (.alivetime _playerstatus)) "; Name: " (Variables|/Script/Engine.PlayerState|GetPlayerName (.playerstate _playerstatus)))))

(fn PrintAllActorClasses
  (bind _outactors (Actor|GetAllActorsOfClass "/Script/Engine.Actor"))
  (for _array_element _outactors
    (Utilities|Set|Add (LocalVariables|GetuniqueNames) (Utilities|GetClassDisplayName (Utilities|GetClass _array_element))))
  (bind _result (Utilities|Set|ToArray (LocalVariables|GetuniqueNames)))
  (for _array_element_2 _result
    (CallFunction|PrintDebug _array_element_2)))