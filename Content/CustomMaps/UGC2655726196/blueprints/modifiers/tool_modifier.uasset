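; Pavlov multi-tool modifier attached to a held taser, offering class registering and spawning, map loading and teleporting, target or bot spawning, noclip, ruler and debug settings.
; Tick detects the holding hand to enable that hand actor's input, drives noclip and ruler updates, and self-destroys when detached.
; Actions dispatch on a cyclable enum with per-action sub-options shown on a TextRender.
; Maps stream in as offset level instances, with shared state in GameLogic.
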(event Custom|Start%20Ruler
  (Variables|Default|SetMeasuring true)
  (Transformation|DetachFromComponent (Variables|Default|GetRulerPoint) "KeepWorld" "KeepWorld" "KeepWorld" true))

(event Custom|EndRuler
  (Variables|Default|SetMeasuring false)
  (Transformation|AttachComponentToComponent (Variables|Default|GetRulerPoint) (Variables|Default|GetDefaultSceneRoot) "None" "SnapToTarget" "SnapToTarget" "SnapToTarget" true)
  (CallFunction|UpdateDisplay))

(event Custom|CycleMap
  (bind _outrownames (DataTable|GetDataTableRowNames "/Game/CustomMaps/UGC2655726196/blueprints/modifiers/enums/MapList.MapList"))
  (bind _returnvalue (Utilities|GetDataTableRow "/Game/CustomMaps/UGC2655726196/blueprints/modifiers/enums/MapList.MapList" (Utilities|Array|Get(acopy) _outrownames (Math|Integer|%(Integer) (+ (Variables|Default|GetMapIndex) 1) (Utilities|Array|Length _outrownames))))
    (:then
      (Variables|Default|SetCurMap _returnvalue)
      (Variables|Default|SetMapIndex (Math|Integer|%(Integer) (+ (Variables|Default|GetMapIndex) 1) (Utilities|Array|Length _outrownames))))))

(event Custom|InitMap
  (bind _outrownames (DataTable|GetDataTableRowNames "/Game/CustomMaps/UGC2655726196/blueprints/modifiers/enums/MapList.MapList"))
  (bind _returnvalue (Utilities|GetDataTableRow "/Game/CustomMaps/UGC2655726196/blueprints/modifiers/enums/MapList.MapList" (Utilities|Array|Get(acopy) _outrownames))
    (:then
      (Variables|Default|SetCurMap _returnvalue)
      (Variables|Default|SetMapIndex 0))))

(event EventBeginPlay
  (CallFunction|InitMap))

(event EventTick
  (params (DeltaSeconds :type Float%20%28single-precision%29))
  (bind _returnvalue (Game|GetPlayerController 0))
  (bind _returnvalue_2 (Game|Player|GetPlayerPawn 0))
  (bind _returnvalue_3 (Actor|GetAttachParentActor))
  (bind _returnvalue_4 (Actor|GetAttachParentActor _returnvalue_3))
  (Utilities|FlowControl|Sequence
    (:then_0
      ;[1 1 1] Check if the tool is being held / in inventory and also destroy it if the taser it's attached to despawns.
      (Utilities|IsValid _returnvalue_3
        (:Is%20Valid
          (switch string (Utilities|GetClassDisplayName (Utilities|GetClass _returnvalue_4))
            (:Default
              (Input|DisableInput (Variables|Default|GetLeftHand_ref) _returnvalue :!label _label)
              (Input|DisableInput (Variables|Default|GetRightHand_ref) _returnvalue)
              (if (Variables|Default|GetinHand)
                (CallFunction|OnToolDropped)
                (Variables|Default|SetinHand false)))
            (:BP_PavlovController_C
              (bind _right_hand (CallFunction|GetHands (Pawn|GetControlledPawn _returnvalue)))
              (Variables|Default|SetinHand true)
              (bind _output_get (Variables|Default|SetinRightHand (== _returnvalue_4 (Components|GetOwner _right_hand))))
              (if _output_get
                (Input|EnableInput (Variables|Default|GetRightHand_ref) _returnvalue)
                (else
                  (Input|EnableInput (Variables|Default|GetLeftHand_ref) _returnvalue))))
            (:BP_PavlovInventory_C
              (goto _label))))
        (:Is%20Not%20Valid
          (Actor|DestroyActor))))
    (:then_1
      ;[1 1 1] Noclip tick
      (if (Variables|Default|GetnoclipFlying)
        (Transformation|SetActorLocation _returnvalue_2 (+ (Transformation|GetActorLocation _returnvalue_2) (* (Math|Vector|GetForwardVector (Variables|Default|GetFireDirection)) (* DeltaSeconds 2e+03))) false true)))
    (:then_2
      (if (and (Variables|Default|GetMeasuring) (Utilities|Enum|Equal(Enum) (Variables|Default|GetcurAction) "NewEnumerator11"))
        (CallFunction|UpdateDisplay)))))

(fn ConstructionScript
  (bind _self self)
  (bind _asentity_info (Utilities|Casting|CastToentity_info (Variables|/Script/Engine.ChildActorComponent|GetChildActor (Variables|Default|GetEntityInfo))))
  (bind _output_get (Variables|Default|SetEntityInfo_ref _asentity_info))
  (Variables|/Game/CustomMaps/UGC2655726196/blueprints/entity_info.entity_info_C|Setwhitelist _output_get true)
  (Default|Clear _output_get)
  (CallFunction|UpdateDisplay)
  (Utilities|FlowControl|Sequence
    (:then_0
      (bind _astool_hand_right (Utilities|Casting|CastTotool_hand_right (Variables|/Script/Engine.ChildActorComponent|GetChildActor (Variables|Default|GetRightHand))))
      (Variables|/Game/CustomMaps/UGC2655726196/blueprints/modifiers/tool_hand_right.tool_hand_right_C|SettoolModifier _astool_hand_right _self)
      (Variables|Default|SetRightHand_ref _astool_hand_right))
    (:then_1
      (bind _astool_hand_left (Utilities|Casting|CastTotool_hand_left (Variables|/Script/Engine.ChildActorComponent|GetChildActor (Variables|Default|GetLeftHand))))
      (Variables|/Game/CustomMaps/UGC2655726196/blueprints/modifiers/tool_hand_left.tool_hand_left_C|SettoolModifier _astool_hand_left _self)
      (Variables|Default|SetLeftHand_ref _astool_hand_left))))

(fn DoAction
  (params (action%20 :type tool_modifier_actions%20Enum :default "NewEnumerator0") (On :type Boolean))
  (bind _returnvalue (Game|Player|GetPlayerPawn 0))
  (bind _array (Utilities|Array|MakeArray "/Game/Maps/Industry/Industry_Blockout_01.umap" "/Game/Maps/Industry/Industry_Gameplay_01.umap" "/Game/Maps/Industry/Industry_Geo_01.umap" "/Game/Maps/Industry/Industry_Lighting_01.umap" "/Game/Maps/Industry/Industry_Sound_01.umap"))
  (bind _array_2 (Utilities|Array|MakeArray))
  (bind _array_3 (Utilities|Array|MakeArray "/Game/Maps/Santorini/Santorini_Blockout_01.umap" "/Game/Maps/Santorini/Santorini_Gameplay_01.umap" "/Game/Maps/Santorini/Santorini_Geo_01.umap" "/Game/Maps/Santorini/Santorini_Lighting_01.umap" "/Game/Maps/Santorini/Santorini_Sound_01.umap"))
  (bind _mapselected (Variables|Default|GetmapSelected))
  (bind _entityinfo (Variables|Default|GetEntityInfo))
  (bind _curmap (Variables|Default|GetCurMap))
  (bind _curtargetspawnmode (Variables|Default|GetcurTargetSpawnMode))
  (bind _maplocation (Utilities|Struct|BreakLoadableMaps _curmap))
  (bind _returnvalue_2 (Transformation|GetActorLocation _returnvalue))
  (bind _returnvalue_3 (Transformation|GetWorldLocation _entityinfo))
  (bind _returnvalue_4 (Utilities|Select :Index _mapselected :NewEnumerator13 _array_2 :NewEnumerator4 _array_2 :NewEnumerator8 _array_2 :NewEnumerator2 _array :NewEnumerator10 _array_2 :NewEnumerator14 _array_2 :NewEnumerator15 _array_2 :NewEnumerator18 _array_3 :NewEnumerator19 _array_2 :NewEnumerator20 _array_2 :NewEnumerator21 _array_2 :NewEnumerator22 _array_2 :NewEnumerator23 _array_2 :NewEnumerator17 _array_2))
  (bind _z (Math|Vector|BreakVector _returnvalue_3))
  (bind _returnvalue_5 (Math|Rotator|FindLookatRotation _returnvalue_3 (Math|Vector|MakeVector (.x _returnvalue_2) (.y _returnvalue_2) _z)))
  (bind _returnvalue_6 (Math|Transform|MakeTransform _returnvalue_3 _returnvalue_5))
  (if On
    (switch Utilities|FlowControl|Switch|Switchontool_modifier_actions action%20
      (:NewEnumerator0
        ;[1 1 1] Register Class
        (bind _result (Utilities|Set|ToArray (Variables|/Game/CustomMaps/UGC2655726196/blueprints/entity_info.entity_info_C|GetActorRefs (Variables|Default|GetEntityInfo_ref))))
        (for _array_element _result
          (Utilities|Array|AddUnique (Variables|Default|Getregistered_classes) (Utilities|GetClass _array_element))))
      (:NewEnumerator1
        ;[1 1 1] Spawn Selected Class
        (Game|SpawnActorfromClass (Utilities|GetCurClass) (Math|Transform|MakeTransform (Transformation|GetWorldLocation (Variables|Default|GetEntityInfo))) "Undefined" 0 0))
      (:NewEnumerator6
        ;[1 1 1] Load Map
        (bind _gamelogic (Utilities|GetGameLogic)
          (:ExecOut
            (if (Variables|/Game/CustomMaps/UGC2655726196/blueprints/gamelogic.gamelogic_C|GetmapLoaded _gamelogic)
              (CallFunction|DoMapLoadedAction)
              (else
                (bind _offs (CallFunction|GetMapOffset _maplocation))
                (bind (_boutsuccess _returnvalue_7) (Class|LevelStreamingDynamic|LoadLevelInstance (Utilities|String|Trim _maplocation) (+ _offs (Math|Vector|MakeVector 0.0 0.0 0.0)) "0, 0, 0"))
                (bind _output_get (Variables|/Game/CustomMaps/UGC2655726196/blueprints/gamelogic.gamelogic_C|SetmapLoaded _gamelogic _boutsuccess))
                (Variables|/Game/CustomMaps/UGC2655726196/blueprints/gamelogic.gamelogic_C|SetmapRef _gamelogic _returnvalue_7)
                (if _output_get
                  (if (> (Utilities|Array|Length _returnvalue_4) 0)
                    (for _array_element_2 _returnvalue_4
                      (Class|LevelStreamingDynamic|LoadLevelInstance _array_element_2 (+ _offs (Math|Vector|MakeVector 0.0 0.0 0.0)) "0, 0, 0")))
                  (CallFunction|UpdateDisplay)
                  (bind _outactors (Actor|GetAllActorsOfClass "/Engine/EngineSky/BP_Sky_Sphere.BP_Sky_Sphere_C"))
                  (Rendering|SetActorHiddenInGame (Utilities|Array|Get(acopy) _outactors) true)))))))
      (:NewEnumerator7
        ;[1 1 1] Spawn Box
        (LocalVariables|SetdeletedTarget false)
        (bind _result_2 (Utilities|Set|ToArray (Variables|/Game/CustomMaps/UGC2655726196/blueprints/entity_info.entity_info_C|GetActorRefs (Variables|Default|GetEntityInfo_ref))))
        (for _array_element_3 _result_2
          (if (Utilities|String|Contains (Utilities|GetClassDisplayName (Utilities|GetClass _array_element_3)) "Target")
            (LocalVariables|SetdeletedTarget true)
            (Actor|DestroyActor _array_element_3)))
        (if (not (LocalVariables|GetdeletedTarget))
          (if (Utilities|Enum|Equal(Enum) _curtargetspawnmode "NewEnumerator2")
            (CallFunction|SpawnBot _returnvalue_6)
            (else
              (Game|SpawnActorfromClass (.Value (Utilities|Map|Find (Variables|Default|GetTargetSpawnModeLookup) _curtargetspawnmode)) _returnvalue_6 "Undefined" 0 0)))))
      (:NewEnumerator8
        ;[1 1 1] Noclip
        (bind _output_get_2 (Variables|Default|SetnoclipFlying On :!label _label))
        (switch Utilities|FlowControl|Switch|Switchonnoclip_mode (Variables|Default|GetcurNoclipMode)
          (:NewEnumerator0
            (CallFunction|UpdateNoclip _output_get_2))))
      (:NewEnumerator10
        (CallFunction|DoSetting))
      (:NewEnumerator11
        (if (Variables|Default|GetMeasuring)
          (CallFunction|EndRuler)
          (else
            (CallFunction|StartRuler)))))
    (else
      (switch Utilities|FlowControl|Switch|Switchontool_modifier_actions action%20
        (:NewEnumerator8
          (goto _label))))))

(fn CycleAction
  (CallFunction|OnCyclefrom (Variables|Default|GetcurAction))
  (Variables|Default|SetcurAction (Utilities|Enum|ByteToEnumtool_modifier_actions (Utilities|CycleEnum (Variables|Default|GetcurAction) (|GetNumEnumEntries))))
  (CallFunction|UpdateDisplay))

(fn UpdateDisplay
  (bind _rulerpoint (Variables|Default|GetRulerPoint))
  (bind _firedirection (Variables|Default|GetFireDirection))
  (bind _currulermode (Variables|Default|GetcurRulerMode))
  (bind _cursetting (Variables|Default|GetcurSetting))
  (bind _returnvalue (Transformation|GetWorldLocation _rulerpoint))
  (bind _returnvalue_2 (Transformation|GetWorldLocation _firedirection))
  (bind _returnvalue_3 (Utilities|Select :Index _currulermode :NewEnumerator0 "Ruler 3D" :NewEnumerator1 "Ruler 2D"))
  (LocalVariables|Setbuffer (Utilities|String|EnumtoString (Variables|Default|GetcurAction)))
  (Rendering|SetVisibility (Variables|Default|GetEntityInfo) (or (Utilities|Enum|Equal(Enum) (Variables|Default|GetcurAction) "NewEnumerator0") (Utilities|Enum|Equal(Enum) (Variables|Default|GetcurAction) "NewEnumerator7")) true)
  (Utilities|FlowControl|Sequence
    (:then_0
      (switch Utilities|FlowControl|Switch|Switchontool_modifier_actions (Variables|Default|GetcurAction)
        (:NewEnumerator1
          (LocalVariables|Settmp (Utilities|GetClassDisplayName (Utilities|GetCurClass)))
          (LocalVariables|Setbuffer (Utilities|String|Append (LocalVariables|Getbuffer) " 
< " (stale _output_get) " >") :!label _label))
        (:NewEnumerator6
          (bind _gamelogic (Utilities|GetGameLogic)
            (:ExecOut
              (if (Variables|/Game/CustomMaps/UGC2655726196/blueprints/gamelogic.gamelogic_C|GetmapLoaded _gamelogic)
                (LocalVariables|Settmp (Utilities|String|EnumtoString (Variables|Default|GetcurMapLoadedAction)))
                (goto _label)
                (else
                  (LocalVariables|Settmp (.MapName (Utilities|Struct|BreakLoadableMaps (Variables|Default|GetCurMap))))
                  (goto _label))))))
        (:NewEnumerator7
          (LocalVariables|Settmp (Utilities|String|EnumtoString (Variables|Default|GetcurTargetSpawnMode)))
          (goto _label))
        (:NewEnumerator8
          (bind _output_get (LocalVariables|Settmp (Utilities|String|EnumtoString (Variables|Default|GetcurNoclipMode))))
          (goto _label))
        (:NewEnumerator10
          (bind _rep (CallFunction|GetSettingValue _cursetting))
          (LocalVariables|Setbuffer (Utilities|String|Append (LocalVariables|Getbuffer) " 
< " (Utilities|String|EnumtoString _cursetting) " >: " _rep)))
        (:NewEnumerator11
          (if (Variables|Default|GetMeasuring)
            (LocalVariables|Setbuffer (Utilities|String|Append _returnvalue_3 " 
< " (Utilities|String|ToString(Text) (Utilities|Text|ToText(Float) (Utilities|Select :Index (Variables|Default|GetcurRulerMode) :NewEnumerator0 (/ (Math|Vector|VectorLength (- _returnvalue_2 _returnvalue)) 1e+02) :NewEnumerator1 (/ (Math|Vector|VectorLength (- (* _returnvalue_2 "1.000000,1.000000, 0") (* _returnvalue "1.000000,1.000000, 0"))) 1e+02)) "HalfToEven" false true 1 324 2 2)) "m>"))
            (else
              (LocalVariables|Setbuffer _returnvalue_3))))))
    (:then_5
      (Rendering|Components|TextRender|SetText (Variables|Default|GetTextRender) (Utilities|Text|ToText(String) (LocalVariables|Getbuffer))))))

(fn DebugPrintParents
  (bind _output_get (LocalVariables|Setparent self))
  (LocalVariables|Setbuffer "")
  (while (Utilities|IsValid _output_get)
    (LocalVariables|Setbuffer (Utilities|String|Append (Utilities|GetClassDisplayName (Utilities|GetClass (LocalVariables|Getparent))) " 
" (LocalVariables|Getbuffer)))
    (LocalVariables|Setparent (Actor|GetAttachParentActor (LocalVariables|Getparent))))
  (Rendering|Components|TextRender|SetText (Variables|Default|GetTextRender) (Utilities|Text|ToText(String) (LocalVariables|Getbuffer))))

(fn CycleSecondaryAction
  (Utilities|FlowControl|Sequence
    (:then_0
      (switch Utilities|FlowControl|Switch|Switchontool_modifier_actions (Variables|Default|GetcurAction)
        (:NewEnumerator1
          (Variables|Default|SetcurClassIdx (Math|Conversions|ToInteger(Byte) (Utilities|CycleEnum (Math|Conversions|ToByte(Integer) (Variables|Default|GetcurClassIdx)) (Utilities|Array|Length (Variables|Default|Getregistered_classes))))))
        (:NewEnumerator6
          (bind _gamelogic (Utilities|GetGameLogic)
            (:ExecOut
              (if (Variables|/Game/CustomMaps/UGC2655726196/blueprints/gamelogic.gamelogic_C|GetmapLoaded _gamelogic)
                (Variables|Default|SetcurMapLoadedAction (Utilities|Enum|ByteToEnummap_loaded_actions (Utilities|CycleEnum (Variables|Default|GetcurMapLoadedAction) (|GetNumEnumEntries))))
                (else
                  (CallFunction|CycleMap))))))
        (:NewEnumerator7
          (Variables|Default|SetcurTargetSpawnMode (Utilities|Enum|ByteToEnumtarget_spawn_mode (Utilities|CycleEnum (Variables|Default|GetcurTargetSpawnMode) (|GetNumEnumEntries)))))
        (:NewEnumerator8
          (bind _output_get (Variables|Default|SetcurNoclipMode (Utilities|Enum|ByteToEnumnoclip_mode (Utilities|CycleEnum (Variables|Default|GetcurNoclipMode) (|GetNumEnumEntries)))))
          (CallFunction|UpdateNoclip (Utilities|Enum|Equal(Enum) _output_get "NewEnumerator1")))
        (:NewEnumerator10
          (Variables|Default|SetcurSetting (Utilities|Enum|ByteToEnumsettings_actions (Utilities|CycleEnum (Variables|Default|GetcurSetting) (|GetNumEnumEntries)))))
        (:NewEnumerator11
          (Variables|Default|SetcurRulerMode (Utilities|Enum|ByteToEnumruler_modes (Utilities|CycleEnum (Variables|Default|GetcurRulerMode) (|GetNumEnumEntries)))))))
    (:then_1
      (CallFunction|UpdateDisplay))))

(fn GetSafeSpawnPoint
  (params (startPoint :type Vector) (StartArea :type Boolean))
  (bind (_x _y) (Math|Vector|BreakVector startPoint))
  (bind _outactors (Actor|GetAllActorsOfClass "/Script/PavlovProxy.Pavlov_Spawn"))
  (bind _array_element (Utilities|Array|ForEachLoopwithBreak _outactors :!label _label)
    (:LoopBody
      (if StartArea
        (if (Utilities|Name|Equal(Name) (Variables|/Script/Engine.PlayerStart|GetPlayerStartTag _array_element) "Start")
          (LocalVariables|SetSpawn _array_element :!label _label_2)
          (goto _label Break))
        (elif (Utilities|Name|NotEqual(Name) (Variables|/Script/Engine.PlayerStart|GetPlayerStartTag _array_element) "Start")
          (goto _label_2))))
    (:Completed
      (bind _spawn (LocalVariables|GetSpawn)
        (:then
          (return (Transformation|GetActorLocation _spawn) true))
        (:else
          (bind (_outhit _returnvalue) (Collision|LineTraceByChannel startPoint (Math|Vector|MakeVector _x _y 0.0) "TraceTypeQuery1" false 0 "None"))
          (return (+ (.impactpoint _outhit) "0, 0,500.000000") _returnvalue))))))

(fn SpawnBot
  (params (transform :type Transform))
  (bind _returnvalue (AI|SpawnAIFromClass (Utilities|GetClass (Game|Player|GetPlayerPawn 0)) "/Game/CustomMaps/UGC2655726196/blueprints/modifiers/bot_ai/bot_bt.bot_bt" (.location transform) (.rotation transform) false))
  (Variables|/Script/AIModule.AIController|SetbStopAILogicOnUnposses (AI|GetAIController _returnvalue) true)
  (Pawn|UnPossess (AI|GetAIController _returnvalue))
  (Actor|DestroyActor (AI|GetAIController _returnvalue))
  (bind _returnvalue_2 (Game|SpawnActorfromClass "/Game/CustomMaps/UGC2655726196/blueprints/modifiers/bot_ai/bot_controller.bot_controller_C" transform "Undefined" 0 0))
  (Pawn|Possess _returnvalue_2 _returnvalue)
  (Transformation|SetActorLocation _returnvalue (.location transform) false false)
  (AI|RunBehaviorTree _returnvalue_2 "/Game/CustomMaps/UGC2655726196/blueprints/modifiers/bot_ai/bot_bt.bot_bt"))

(fn DoMapLoadedAction
  (switch Utilities|FlowControl|Switch|Switchonmap_loaded_actions (Variables|Default|GetcurMapLoadedAction)
    (:NewEnumerator0
      (bind (_spawnloc _tracesuccessful) (CallFunction|GetSafeSpawnPoint "0.000000,0.000000,100000.000000" false))
      (if _tracesuccessful
        (Transformation|SetActorLocation (Game|Player|GetPlayerPawn 0) _spawnloc false true)
        (else
          (bind _gamelogic (Utilities|GetGameLogic)
            (:ExecOut
              (Default|Print _gamelogic "Map has not finished loading.")
              (Default|Print _gamelogic (Utilities|String|ToString(Vector) (Transformation|GetActorLocation (Pawn|GetControlledPawn (Game|GetPlayerController 0))))))))))
    (:NewEnumerator1
      (bind _spawnloc_2 (CallFunction|GetSafeSpawnPoint "299.000000,598.000000,1000.000000" true))
      (Transformation|SetActorLocation (Game|Player|GetPlayerPawn 0) _spawnloc_2 false true))))

(fn UpdateNoclip
  (params (Enabled :type Boolean))
  (bind _returnvalue (Game|Player|GetPlayerPawn 0))
  (bind _returnvalue_2 (not Enabled))
  (bind _returnvalue_3 (Pawn|GetMovementComponent _returnvalue))
  (Collision|SetActorEnableCollision _returnvalue _returnvalue_2)
  (Variables|/Script/Engine.MovementComponent|SetVelocity _returnvalue_3 "0, 0, 0")
  (Components|Activation|SetActive _returnvalue_3 _returnvalue_2 true))

(fn OnToolDropped
  (switch Utilities|FlowControl|Switch|Switchontool_modifier_actions (Variables|Default|GetcurAction)
    (:NewEnumerator8
      (CallFunction|UpdateNoclip false)
      (CallFunction|DoAction "NewEnumerator8" false))))

(fn OnCyclefrom
  (params (action :type tool_modifier_actions%20Enum :default "NewEnumerator0"))
  (switch Utilities|FlowControl|Switch|Switchontool_modifier_actions action
    (:NewEnumerator8
      (CallFunction|UpdateNoclip false)
      (CallFunction|DoAction "NewEnumerator8" false))
    (:NewEnumerator11
      (CallFunction|EndRuler))))

(fn DoSetting
  (bind _cursetting (Variables|Default|GetcurSetting))
  (bind _gamelogic (Utilities|GetGameLogic)
    (:ExecOut
      (Utilities|Map|Add (Variables|/Game/CustomMaps/UGC2655726196/blueprints/gamelogic.gamelogic_C|GetboolSettings _gamelogic) _cursetting (not (.Value (Utilities|Map|Find (Variables|/Game/CustomMaps/UGC2655726196/blueprints/gamelogic.gamelogic_C|GetboolSettings _gamelogic) _cursetting))))
      (CallFunction|UpdateDisplay)
      (switch Utilities|FlowControl|Switch|Switchonsettings_actions _cursetting
        (:NewEnumerator0
          (if (not (.Value (Utilities|Map|Find (Variables|/Game/CustomMaps/UGC2655726196/blueprints/gamelogic.gamelogic_C|GetboolSettings _gamelogic) _cursetting)))
            (bind _outactors (Actor|GetAllActorsOfClass "/Game/CustomMaps/UGC2655726196/blueprints/modifiers/grenade_modifier.grenade_modifier_C"))
            (for _array_element _outactors
              (Actor|DestroyActor _array_element))))
        (:NewEnumerator1
          (if (.Value (Utilities|Map|Find (Variables|/Game/CustomMaps/UGC2655726196/blueprints/gamelogic.gamelogic_C|GetboolSettings _gamelogic) _cursetting))
            (bind _outactors_2 (Actor|GetAllActorsOfClass "/Script/Engine.PlayerStart"))
            (for _array_element_2 _outactors_2
              (Game|SpawnActorfromClass "/Game/CustomMaps/UGC2655726196/blueprints/modifiers/spawn_modifier.spawn_modifier_C" (Math|Transform|MakeTransform (Transformation|GetActorLocation _array_element_2) "0, 0, 0" "1,1,1") "Undefined" 0 0))
            (else
              (bind _outactors_3 (Actor|GetAllActorsOfClass "/Game/CustomMaps/UGC2655726196/blueprints/modifiers/spawn_modifier.spawn_modifier_C"))
              (for _array_element_3 _outactors_3
                (Actor|DestroyActor _array_element_3)))))
        (:NewEnumerator2
          (if (.Value (Utilities|Map|Find (Variables|/Game/CustomMaps/UGC2655726196/blueprints/gamelogic.gamelogic_C|GetboolSettings _gamelogic) _cursetting))
            (bind _outactors_4 (Actor|GetAllActorsOfClass "/Script/Engine.StaticMeshActor"))
            (for _array_element_4 _outactors_4
              (for _index (range 0 (- (Rendering|Material|GetNumMaterials (Variables|/Script/Engine.StaticMeshActor|GetStaticMeshComponent _array_element_4)) 1))
                (bind _penetrable (CallFunction|IsSurfacePenetrable (Variables|/Script/Engine.PhysicalMaterial|GetSurfaceType (Class|MaterialInterface|GetPhysicalMaterial (Rendering|Material|GetMaterial (Variables|/Script/Engine.StaticMeshActor|GetStaticMeshComponent _array_element_4) _index)))))
                (if _penetrable
                  (Game|SpawnActorfromClass "/Game/CustomMaps/UGC2655726196/blueprints/modifiers/penmat_modifier.penmat_modifier_C" (Math|Transform|MakeTransform (Transformation|GetWorldLocation (Variables|/Script/Engine.StaticMeshActor|GetStaticMeshComponent _array_element_4)) "0, 0, 0" "1,1,1") "Undefined" 0 (Variables|/Script/Engine.StaticMeshActor|GetStaticMeshComponent _array_element_4) _index 0))))
            (else
              (bind _outactors_5 (Actor|GetAllActorsOfClass "/Game/CustomMaps/UGC2655726196/blueprints/modifiers/penmat_modifier.penmat_modifier_C"))
              (for _array_element_5 _outactors_5
                (Actor|DestroyActor _array_element_5)))))))))

(fn GetSettingValue
  (params (setting :type settings_actions%20Enum :default "NewEnumerator0"))
  (bind _gamelogic (Utilities|GetGameLogic)
    (:ExecOut
      (bind _on_off (Utilities|BooltoonOff (.Value (Utilities|Map|Find (Variables|/Game/CustomMaps/UGC2655726196/blueprints/gamelogic.gamelogic_C|GetboolSettings _gamelogic) setting)))
        (:Out
          (return _on_off))))))

(fn IsSurfacePenetrable
  (params (surfaceType :type EPhysicalSurface%20Enum :default "SurfaceType_Default"))
  (switch Utilities|FlowControl|Switch|SwitchonEPhysicalSurface surfaceType
    (:SurfaceType_Default
      _)
    (:SurfaceType1
      _)
    (:SurfaceType2
      _)
    (:SurfaceType3
      _)
    (:SurfaceType4
      _)
    (:SurfaceType5
      _)
    (:SurfaceType6
      _)
    (:SurfaceType7
      _)
    (:SurfaceType8
      _)
    (:SurfaceType9
      _)
    (:SurfaceType10
      _)
    (:SurfaceType11
      _)
    (:SurfaceType33
      (return true))
    (:SurfaceType34
      (return true))
    (:SurfaceType35
      (return true))
    (:SurfaceType36
      (return true))
    (:SurfaceType37
      (return true))
    (:SurfaceType38
      (return true))
    (:SurfaceType39
      (return true))
    (:SurfaceType40
      (return true))
    (:SurfaceType41
      (return true)))
  (return false))

(fn GetMapOffset
  (params (map :type String))
  (bind _mapoffsets (Variables|Default|GetmapOffsets))
  (bind (_value _returnvalue) (Utilities|Map|Find _mapoffsets map))
  (if _returnvalue
    (return _value)
    (else
      (return "0, 0, 0"))))