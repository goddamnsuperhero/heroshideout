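; Left-hand input relay for a VR tool modifier, mapping left controller buttons to the tool's actions.
; Trigger press and release switch the ToolModifier's current action on and off.
; The fire mode button cycles the primary action, while the magazine release and bolt release buttons both cycle the secondary action.
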(event Input|ActionEvents|InputActionMagBoltReleaseLeft
  (params (Key :type Key%20Structure))
  (:Pressed
    (Default|CycleSecondaryAction (Variables|Default|GettoolModifier))))

(event Input|ActionEvents|InputActionCycleFireModeLeft
  (params (Key :type Key%20Structure))
  (:Pressed
    (Default|CycleAction (Variables|Default|GettoolModifier))))

(event Input|ActionEvents|InputActionTriggerLeft
  (params (Key :type Key%20Structure))
  (bind _toolmodifier (Variables|Default|GettoolModifier))
  (bind _curaction (Variables|/Game/CustomMaps/UGC2655726196/blueprints/modifiers/tool_modifier.tool_modifier_C|GetcurAction _toolmodifier))
  (:Pressed
    (Default|DoAction _toolmodifier _curaction true))
  (:Released
    (Default|DoAction _toolmodifier _curaction false)))

(event Input|ActionEvents|InputActionReleaseMagazineLeft
  (params (Key :type Key%20Structure))
  (:Pressed
    (Default|CycleSecondaryAction (Variables|Default|GettoolModifier))))

(fn ConstructionScript)