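; Loot spawner Blueprint that shows a model of its configured loot, such as weapons, grenades, tools, attachments and armour.
; The construction script rebuilds SpawnList as unique strings from LootSpawnEnums, when that array is non-empty, then runs the parent construction script.
; A hardcoded string-to-mesh chain then sets the Item mesh for each entry, so the last recognised entry wins.
; It has no active runtime logic of its own.
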(event EventBeginPlay)

(event Collision|EventActorBeginOverlap
  (params (OtherActor :type Actor%20Object%20Reference)))

(event EventTick
  (params (DeltaSeconds :type Float%20%28single-precision%29)))

(fn ConstructionScript
  (Utilities|FlowControl|Sequence
    (:then_0
      (if (> (Utilities|Array|Length (Variables|Default|GetLootSpawnEnums)) 0)
        (Utilities|Array|Clear (Variables|Default|GetSpawnList))
        (for _array_element (Variables|Default|GetLootSpawnEnums)
          (Utilities|Array|AddUnique (Variables|Default|GetSpawnList) (Utilities|String|EnumtoString _array_element))))
      (|CallParentFunction))
    (:then_1
      (for _array_element_2 (Variables|Default|GetSpawnList)
        (Utilities|FlowControl|Sequence
          (:then_0
            (if (Utilities|Enum|Equal(Enum) _array_element_2 "knife")
              (Components|StaticMesh|SetStaticMesh (Variables|Default|GetItem) "/Game/CustomMaps/UGC2655726196/external/weapons_pack/Props/Knife.Knife")))
          (:then_1
            (if (Utilities|Enum|Equal(Enum) _array_element_2 "cet9")
              (Components|StaticMesh|SetStaticMesh (Variables|Default|GetItem) "/Game/CustomMaps/UGC2655726196/external/weapons_pack/Props/Cet9.Cet9")))
          (:then_2
            (if (Utilities|Enum|Equal(Enum) _array_element_2 "m9")
              (Components|StaticMesh|SetStaticMesh (Variables|Default|GetItem) "/Game/CustomMaps/UGC2655726196/external/weapons_pack/Props/M9.M9")))
          (:then_3
            (if (Utilities|Enum|Equal(Enum) _array_element_2 "1911")
              (Components|StaticMesh|SetStaticMesh (Variables|Default|GetItem) "/Game/CustomMaps/UGC2655726196/external/weapons_pack/Props/C1911.C1911")))
          (:then_4
            (if (Utilities|Enum|Equal(Enum) _array_element_2 "sock")
              (Components|StaticMesh|SetStaticMesh (Variables|Default|GetItem) "/Game/CustomMaps/UGC2655726196/external/weapons_pack/Props/Sock.Sock")))
          (:then_5
            (if (Utilities|Enum|Equal(Enum) _array_element_2 "57")
              (Components|StaticMesh|SetStaticMesh (Variables|Default|GetItem) "/Game/CustomMaps/UGC2655726196/external/weapons_pack/Props/57.57")))
          (:then_6
            (if (Utilities|Enum|Equal(Enum) _array_element_2 "de")
              (Components|StaticMesh|SetStaticMesh (Variables|Default|GetItem) "/Game/CustomMaps/UGC2655726196/external/weapons_pack/Props/DE.DE")))
          (:then_7
            (if (Utilities|Enum|Equal(Enum) _array_element_2 "revolver")
              (Components|StaticMesh|SetStaticMesh (Variables|Default|GetItem) "/Game/CustomMaps/UGC2655726196/external/weapons_pack/Props/Revolver.Revolver")))
          (:then_8
            (if (Utilities|Enum|Equal(Enum) _array_element_2 "sawedoff")
              (Components|StaticMesh|SetStaticMesh (Variables|Default|GetItem) "/Game/CustomMaps/UGC2655726196/external/weapons_pack/Props/Sawedoff.Sawedoff")))
          (:then_9
            (if (Utilities|Enum|Equal(Enum) _array_element_2 "shotgun")
              (Components|StaticMesh|SetStaticMesh (Variables|Default|GetItem) "/Game/CustomMaps/UGC2655726196/external/weapons_pack/Props/PumpShotgun.PumpShotgun")))
          (:then_10
            (if (Utilities|Enum|Equal(Enum) _array_element_2 "autoshotgun")
              (Components|StaticMesh|SetStaticMesh (Variables|Default|GetItem) "/Game/CustomMaps/UGC2655726196/external/weapons_pack/Props/CombatShotgun.CombatShotgun")))
          (:then_11
            (if (Utilities|Enum|Equal(Enum) _array_element_2 "drumshotgun")
              (Components|StaticMesh|SetStaticMesh (Variables|Default|GetItem) "/Game/CustomMaps/UGC2655726196/external/weapons_pack/Props/DrumShotgun.DrumShotgun")))
          (:then_12
            (if (Utilities|Enum|Equal(Enum) _array_element_2 "lmga")
              (Components|StaticMesh|SetStaticMesh (Variables|Default|GetItem) "/Game/CustomMaps/UGC2655726196/external/weapons_pack/Props/LMG_A.LMG_A")))
          (:then_13
            (if (Utilities|Enum|Equal(Enum) _array_element_2 "uzi")
              (Components|StaticMesh|SetStaticMesh (Variables|Default|GetItem) "/Game/CustomMaps/UGC2655726196/external/weapons_pack/Props/Uzi.Uzi")))
          (:then_14
            (if (Utilities|Enum|Equal(Enum) _array_element_2 "mp5")
              (Components|StaticMesh|SetStaticMesh (Variables|Default|GetItem) "/Game/CustomMaps/UGC2655726196/external/weapons_pack/Props/MP5.MP5")))
          (:then_15
            (if (Utilities|Enum|Equal(Enum) _array_element_2 "ak")
              (Components|StaticMesh|SetStaticMesh (Variables|Default|GetItem) "/Game/CustomMaps/UGC2655726196/external/weapons_pack/Props/Bizon.Bizon")))
          (:then_16
            (if (Utilities|Enum|Equal(Enum) _array_element_2 "smg")
              (Components|StaticMesh|SetStaticMesh (Variables|Default|GetItem) "/Game/CustomMaps/UGC2655726196/external/weapons_pack/Props/UMP.UMP")))
          (:then_17
            (if (Utilities|Enum|Equal(Enum) _array_element_2 "vanas")
              (Components|StaticMesh|SetStaticMesh (Variables|Default|GetItem) "/Game/CustomMaps/UGC2655726196/external/weapons_pack/Props/Vanas.Vanas")))
          (:then_18
            (if (Utilities|Enum|Equal(Enum) _array_element_2 "p90")
              (Components|StaticMesh|SetStaticMesh (Variables|Default|GetItem) "/Game/CustomMaps/UGC2655726196/external/weapons_pack/Props/P90.P90")))
          (:then_19
            (if (Utilities|Enum|Equal(Enum) _array_element_2 "kar98")
              (Components|StaticMesh|SetStaticMesh (Variables|Default|GetItem) "/Game/CustomMaps/UGC2655726196/external/weapons_pack/Props/Kar98.Kar98")))
          (:then_20
            (if (Utilities|Enum|Equal(Enum) _array_element_2 "ak47")
              (Components|StaticMesh|SetStaticMesh (Variables|Default|GetItem) "/Game/CustomMaps/UGC2655726196/external/weapons_pack/Props/AK47.AK47")))
          (:then_21
            (if (Utilities|Enum|Equal(Enum) _array_element_2 "ak12")
              (Components|StaticMesh|SetStaticMesh (Variables|Default|GetItem) "/Game/CustomMaps/UGC2655726196/external/weapons_pack/Props/AK12.AK12")))
          (:then_22
            (if (Utilities|Enum|Equal(Enum) _array_element_2 "ar")
              (Components|StaticMesh|SetStaticMesh (Variables|Default|GetItem) "/Game/CustomMaps/UGC2655726196/external/weapons_pack/Props/M4.M4")))
          (:then_23
            (if (Utilities|Enum|Equal(Enum) _array_element_2 "aug")
              (Components|StaticMesh|SetStaticMesh (Variables|Default|GetItem) "/Game/CustomMaps/UGC2655726196/external/weapons_pack/Props/AUG.AUG")))
          (:then_24
            (if (Utilities|Enum|Equal(Enum) _array_element_2 "autosniper")
              (Components|StaticMesh|SetStaticMesh (Variables|Default|GetItem) "/Game/CustomMaps/UGC2655726196/external/weapons_pack/Props/AutoSniper.AutoSniper")))
          (:then_25
            (if (Utilities|Enum|Equal(Enum) _array_element_2 "awp")
              (Components|StaticMesh|SetStaticMesh (Variables|Default|GetItem) "/Game/CustomMaps/UGC2655726196/external/weapons_pack/Props/AWP.AWP")))
          (:then_26
            (if (Utilities|Enum|Equal(Enum) _array_element_2 "antitank")
              (Components|StaticMesh|SetStaticMesh (Variables|Default|GetItem) "/Game/CustomMaps/UGC2655726196/external/weapons_pack/Props/AntiTank.AntiTank")))
          (:then_27
            (if (Utilities|Enum|Equal(Enum) _array_element_2 "taser")
              (Components|StaticMesh|SetStaticMesh (Variables|Default|GetItem) "/Game/CustomMaps/UGC2655726196/external/weapons_pack/Props/Taser.Taser")))
          (:then_28
            (if (Utilities|Enum|Equal(Enum) _array_element_2 "grenade")
              (Components|StaticMesh|SetStaticMesh (Variables|Default|GetItem) "/Game/CustomMaps/UGC2655726196/external/weapons_pack/Props/NadeExplosive.NadeExplosive")))
          (:then_29
            (if (Utilities|Enum|Equal(Enum) _array_element_2 "grenade_ru")
              (Components|StaticMesh|SetStaticMesh (Variables|Default|GetItem) "/Game/CustomMaps/UGC2655726196/external/weapons_pack/Props/NadeExplosive_RU.NadeExplosive_RU")))
          (:then_30
            (if (Utilities|Enum|Equal(Enum) _array_element_2 "flash")
              (Components|StaticMesh|SetStaticMesh (Variables|Default|GetItem) "/Game/CustomMaps/UGC2655726196/external/weapons_pack/Props/NadeFlash.NadeFlash")))
          (:then_31
            (if (Utilities|Enum|Equal(Enum) _array_element_2 "flash_ru")
              (Components|StaticMesh|SetStaticMesh (Variables|Default|GetItem) "/Game/CustomMaps/UGC2655726196/external/weapons_pack/Props/NadeFlash_RU.NadeFlash_RU")))
          (:then_32
            (if (Utilities|Enum|Equal(Enum) _array_element_2 "smoke")
              (Components|StaticMesh|SetStaticMesh (Variables|Default|GetItem) "/Game/CustomMaps/UGC2655726196/external/weapons_pack/Props/NadeSmoke.NadeSmoke")))
          (:then_33
            (if (Utilities|Enum|Equal(Enum) _array_element_2 "smoke_ru")
              (Components|StaticMesh|SetStaticMesh (Variables|Default|GetItem) "/Game/CustomMaps/UGC2655726196/external/weapons_pack/Props/NadeSmoke_RU.NadeSmoke_RU")))
          (:then_34
            (if (Utilities|Enum|Equal(Enum) _array_element_2 "painkillers")
              (Components|StaticMesh|SetStaticMesh (Variables|Default|GetItem) "/Game/CustomMaps/UGC2655726196/external/weapons_pack/Props/PillBottle.PillBottle")))
          (:then_35
            (if (Utilities|Enum|Equal(Enum) _array_element_2 "syringe")
              (Components|StaticMesh|SetStaticMesh (Variables|Default|GetItem) "/Game/CustomMaps/UGC2655726196/external/weapons_pack/Props/Syringe.Syringe")))
          (:then_36
            (if (Utilities|Enum|Equal(Enum) _array_element_2 "crowbar")
              (Components|StaticMesh|SetStaticMesh (Variables|Default|GetItem) "/Game/CustomMaps/UGC2655726196/external/weapons_pack/Props/Crowbar.Crowbar")))
          (:then_37
            (if (Utilities|Enum|Equal(Enum) _array_element_2 "handcuffs")
              (Components|StaticMesh|SetStaticMesh (Variables|Default|GetItem) "/Game/CustomMaps/UGC2655726196/external/weapons_pack/Props/Handcuffs.Handcuffs")))
          (:then_38
            (if (Utilities|Enum|Equal(Enum) _array_element_2 "keycard")
              (Components|StaticMesh|SetStaticMesh (Variables|Default|GetItem) "/Game/CustomMaps/UGC2655726196/external/weapons_pack/Props/Keycard.Keycard")))
          (:then_39
            (if (Utilities|Enum|Equal(Enum) _array_element_2 "lockpick")
              (Components|StaticMesh|SetStaticMesh (Variables|Default|GetItem) "/Game/CustomMaps/UGC2655726196/external/weapons_pack/Props/Lockpick.Lockpick")))
          (:then_40
            (if (Utilities|Enum|Equal(Enum) _array_element_2 "pickaxe")
              (Components|StaticMesh|SetStaticMesh (Variables|Default|GetItem) "/Game/CustomMaps/UGC2655726196/external/weapons_pack/Props/Pickaxe.Pickaxe")))
          (:then_41
            (if (Utilities|Enum|Equal(Enum) _array_element_2 "boltcutters")
              (Components|StaticMesh|SetStaticMesh (Variables|Default|GetItem) "/Game/CustomMaps/UGC2655726196/external/weapons_pack/Props/BoltCutters.BoltCutters")))
          (:then_42
            (if (Utilities|Enum|Equal(Enum) _array_element_2 "repairtool")
              (Components|StaticMesh|SetStaticMesh (Variables|Default|GetItem) "/Game/CustomMaps/UGC2655726196/external/weapons_pack/Props/BlowTorch.BlowTorch")))
          (:then_43
            (if (Utilities|Enum|Equal(Enum) _array_element_2 "reddot")
              (Components|StaticMesh|SetStaticMesh (Variables|Default|GetItem) "/Game/CustomMaps/UGC2655726196/external/weapons_pack/Props/RedDot.RedDot")))
          (:then_44
            (if (Utilities|Enum|Equal(Enum) _array_element_2 "holo")
              (Components|StaticMesh|SetStaticMesh (Variables|Default|GetItem) "/Game/CustomMaps/UGC2655726196/external/weapons_pack/Props/Holo.Holo")))
          (:then_45
            (if (Utilities|Enum|Equal(Enum) _array_element_2 "acog")
              (Components|StaticMesh|SetStaticMesh (Variables|Default|GetItem) "/Game/CustomMaps/UGC2655726196/external/weapons_pack/Props/ACOG.ACOG")))
          (:then_46
            (if (Utilities|Enum|Equal(Enum) _array_element_2 "scope")
              (Components|StaticMesh|SetStaticMesh (Variables|Default|GetItem) "/Game/CustomMaps/UGC2655726196/external/weapons_pack/Props/Scope.Scope")))
          (:then_47
            (if (Utilities|Enum|Equal(Enum) _array_element_2 "supp_pistol")
              (Components|StaticMesh|SetStaticMesh (Variables|Default|GetItem) "/Game/CustomMaps/UGC2655726196/external/weapons_pack/Props/SuppressorPistol.SuppressorPistol")))
          (:then_48
            (if (Utilities|Enum|Equal(Enum) _array_element_2 "supp_rifle")
              (Components|StaticMesh|SetStaticMesh (Variables|Default|GetItem) "/Game/CustomMaps/UGC2655726196/external/weapons_pack/Props/SuppressorRifle.SuppressorRifle")))
          (:then_49
            (if (Utilities|Enum|Equal(Enum) _array_element_2 "grip_angled")
              (Components|StaticMesh|SetStaticMesh (Variables|Default|GetItem) "/Game/CustomMaps/UGC2655726196/external/weapons_pack/Props/AngledGrip.AngledGrip")))
          (:then_50
            (if (Utilities|Enum|Equal(Enum) _array_element_2 "grip_vertical")
              (Components|StaticMesh|SetStaticMesh (Variables|Default|GetItem) "/Game/CustomMaps/UGC2655726196/external/weapons_pack/Props/VerticalGrip.VerticalGrip")))
          (:then_51
            (if (Utilities|Enum|Equal(Enum) _array_element_2 "armour")
              (Components|StaticMesh|SetStaticMesh (Variables|Default|GetItem) "/Game/CustomMaps/UGC2655726196/external/weapons_pack/Props/Vest.Vest")))
          (:then_52
            (if (Utilities|Enum|Equal(Enum) _array_element_2 "kevlarhelmet")
              (Components|StaticMesh|SetStaticMesh (Variables|Default|GetItem) "/Game/CustomMaps/UGC2655726196/external/weapons_pack/Props/Helmet.Helmet"))))))))